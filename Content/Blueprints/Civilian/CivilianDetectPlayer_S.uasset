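; Behavior tree service that switches a civilian AI between Patrol and Run based on the player.
; While patrolling, a forward box trace and an eye-level line trace confirm a visible player within SafeDistance before fleeing starts.
; While running, it returns to Patrol once the player is invisible, missing or beyond SafeDistance.
; Transitions write State and PlayerActor to the blackboard and stop current movement.
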(event EventReceiveActivation
  (params (OwnerActor :type Actor%20Object%20Reference))
  (Class|BTFunctionLibrary|SetBlackboardValueasEnum (Variables|Default|GetState)))

(event EventTick
  (params (OwnerActor :type Actor%20Object%20Reference) (DeltaSeconds :type Float%20%28single-precision%29))
  (bind _state (Variables|Default|GetState))
  (bind _playeractor (Variables|Default|GetPlayerActor))
  (bind _returnvalue (Class|BTFunctionLibrary|GetBlackboardValueasEnum _state))
  (bind _returnvalue_2 (Utilities|Enum|ByteToEnumCivilianState _returnvalue))
  (bind _asbp_civilian_ai (Utilities|Casting|CastToBP_CivilianAI OwnerActor))
  (bind _ascivilian (Utilities|Casting|CastToCivilian (Pawn|GetControlledPawn _asbp_civilian_ai)))
  (bind _asmy_character (Utilities|Casting|CastToMyCharacter (Game|Player|GetPlayerPawn 0))
    (:then
      (if (Variables|/Game/Blueprints/Player/MyCharacter.MyCharacter_C|GetisInvisible _asmy_character)
        (switch Utilities|FlowControl|Switch|SwitchonCivilianState _returnvalue_2 :!label _label
          (:NewEnumerator1
            (Class|BTFunctionLibrary|SetBlackboardValueasEnum _state (Utilities|Enum|LiteralenumCivilianState "NewEnumerator0"))
            (Class|BTFunctionLibrary|SetBlackboardValueasObject _playeractor _asmy_character)
            (AI|Navigation|StopMovement _asbp_civilian_ai :!label _label_2)))
        (else
          (switch Utilities|FlowControl|Switch|SwitchonCivilianState (Utilities|Enum|ByteToEnumCivilianState (Class|BTFunctionLibrary|GetBlackboardValueasEnum (Variables|Default|GetState)))
            (:NewEnumerator0
              (bind _outhits (Class|KismetSystemLibrary|BoxTraceMultiforObjects (+ (Transformation|GetActorLocation _ascivilian) (* (Math|Vector|GetForwardVector (Transformation|GetActorRotation _ascivilian)) (.X (Math|Vector|BreakVector (Variables|Default|GetvisionBox))))) (+ (+ (Transformation|GetActorLocation _ascivilian) (* (Math|Vector|GetForwardVector (Transformation|GetActorRotation _ascivilian)) (.X (Math|Vector|BreakVector (Variables|Default|GetvisionBox))))) "1.000000,1.000000,1.000000") (Variables|Default|GetvisionBox) (Transformation|GetActorRotation _ascivilian) (Utilities|Array|MakeArray "ObjectTypeQuery3") false 0 "None" true))
              (Variables|Default|SetplayerInViewRange false)
              (bind _array_element (Utilities|Array|ForEachLoopwithBreak _outhits :!label _label_3)
                (:LoopBody
                  (if (== _asmy_character (.HitActor (Collision|BreakHitResult _array_element)))
                    (Variables|Default|SetplayerInViewRange true)
                    (goto _label_3 Break)))
                (:Completed
                  (if (Variables|Default|GetplayerInViewRange)
                    (bind _outhit (Collision|LineTraceByChannel (+ (Transformation|GetActorLocation _ascivilian) (Math|Vector|MakeVector 0.0 0.0 (Variables|/Script/Engine.Pawn|GetBaseEyeHeight _ascivilian))) (+ (Transformation|GetActorLocation _asmy_character) (Math|Vector|MakeVector 0.0 0.0 (Variables|/Script/Engine.Pawn|GetBaseEyeHeight _asmy_character))) "TraceTypeQuery1" true (Utilities|Array|MakeArray _ascivilian) "None"))
                    (if (== _asmy_character (.HitActor (Collision|BreakHitResult _outhit)))
                      (if (not (> (Math|Float|Absolute(Float) (Math|Vector|VectorLength (- (Transformation|GetActorLocation _asmy_character) (Transformation|GetActorLocation _ascivilian)))) (Variables|Default|GetsafeDistance)))
                        (switch Utilities|FlowControl|Switch|SwitchonCivilianState _returnvalue_2
                          (:NewEnumerator0
                            (Class|BTFunctionLibrary|SetBlackboardValueasEnum _state (Utilities|Enum|LiteralenumCivilianState "NewEnumerator1"))
                            (Class|BTFunctionLibrary|SetBlackboardValueasObject _playeractor _asmy_character)
                            (goto _label_2))))
                      (else
                        (goto _label)))))))
            (:NewEnumerator1
              (if (> (Math|Float|Absolute(Float) (Math|Vector|VectorLength (- (Transformation|GetActorLocation _asmy_character) (Transformation|GetActorLocation _ascivilian)))) (Variables|Default|GetsafeDistance))
                (goto _label)))))))
    (:CastFailed
      (goto _label))))