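; Behavior tree task for civilian AI that picks a random CivilianWaypoint in the level as the next destination.
; It stores a random index in the Route blackboard key, then loops over all waypoints and writes the matching actor's location to Destination.
; The task always finishes as failed, even after setting a destination.
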(event EventReceiveExecute
  (params (OwnerActor :type Actor%20Object%20Reference))
  (bind _outactors (Actor|GetAllActorsOfClass "/Game/Blueprints/Civilian/CivilianWaypoint.CivilianWaypoint_C"))
  (Class|BTFunctionLibrary|SetBlackboardValueasInt (Variables|Default|GetRoute) (Math|Random|RandomIntegerinRange 0 (- (Utilities|Array|Length _outactors) 1)))
  (bind _outactors_2 (Actor|GetAllActorsOfClass "/Game/Blueprints/Civilian/CivilianWaypoint.CivilianWaypoint_C"))
  (for (_array_element _array_index) _outactors_2
    (bind _ascivilian_waypoint (Utilities|Casting|CastToCivilianWaypoint _array_element))
    (if (== _array_index (Class|BTFunctionLibrary|GetBlackboardValueasInt (Variables|Default|GetRoute)))
      (AI|BehaviorTree|SetBlackboardValueasVector (Variables|Default|GetDestination) (Transformation|GetActorLocation _ascivilian_waypoint))))
  (AI|BehaviorTree|FinishExecute false))