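; Behavior tree decorator for civilian AI that advances the Route blackboard value when its node finishes.
; Its condition check always passes, so it acts as a post-execution hook rather than a gate.
; On success it counts all CivilianWaypoint actors and adds a random offset below that count to Route.
; The sum is written back without wrapping or clamping to the waypoint count.
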(event EventReceiveConditionCheck
  (params (OwnerActor :type Actor%20Object%20Reference))
  (Class|BTDecoratorBlueprintBase|FinishConditionCheck true))

(event EventReceiveExecutionFinish
  (params (OwnerActor :type Actor%20Object%20Reference) (NodeResult :type EBTNodeResult%20Enum :default "Succeeded"))
  (bind _route (Variables|Default|GetRoute))
  (bind _outactors (Actor|GetAllActorsOfClass "/Game/Blueprints/Civilian/CivilianWaypoint.CivilianWaypoint_C"))
  (switch Utilities|FlowControl|Switch|SwitchonEBTNodeResult NodeResult
    (:Succeeded
      (Class|BTFunctionLibrary|SetBlackboardValueasInt _route (+ (Class|BTFunctionLibrary|GetBlackboardValueasInt _route) (Math|Random|RandomIntegerinRange 0 (- (Utilities|Array|Length _outactors) 1)))))))