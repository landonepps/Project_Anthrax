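; Policeman AI Blueprint that runs the PoliceBehaviour behavior tree and reacts to noises heard through Pawn Sensing.
; Noises count only when the instigator is tagged as a civilian, policeman, player or possessable object.
; If the blackboard State is Patrol, such a noise switches it to Alerted and stores the noise location as the waypoint.
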(event OnHearNoise(PawnSensing)
  (params (Instigator :type Pawn%20Object%20Reference) (Location :type Vector%20%28by%20ref%29 :default "0, 0, 0") (Volume :type Float%20%28single-precision%29))
  (bind _returnvalue (Utilities|String|StringToName "State"))
  (bind _self self)
  (bind _returnvalue_2 (AI|GetBlackboard _self))
  ;[1 1 1] Set state to alerted when a noise is heard
  (if (Actor|ActorHasTag Instigator "Civilian")
    (switch Utilities|FlowControl|Switch|SwitchonEnemyState (Utilities|Enum|ByteToEnumEnemyState (Class|BlackboardComponent|GetValueasEnum _returnvalue_2 _returnvalue)) :!label _label ; only switch to alerted if in patrol mode
      (:NewEnumerator0
        (AI|Components|Blackboard|SetValueasEnum _returnvalue_2 _returnvalue (Utilities|Enum|LiteralenumEnemyState "NewEnumerator9"))
        (AI|Components|Blackboard|SetValueasVector _returnvalue_2 (Utilities|String|StringToName "waypoint") Location)))
    (elif (Actor|ActorHasTag Instigator "Policeman")
      (goto _label)
      (elif (Actor|ActorHasTag Instigator "Player")
        (goto _label)
        (elif (Actor|ActorHasTag Instigator "Possessable Object")
          (goto _label))))))

(event EventBeginPlay
  (AI|RunBehaviorTree "/Game/Blueprints/Policeman/PoliceBehaviour.PoliceBehaviour"))

(fn ConstructionScript)