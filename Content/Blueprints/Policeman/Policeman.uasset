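; Policeman character Blueprint, a child class that appears to be possessable and is driven by the PoliceBehaviour behavior tree.
; The construction script sets health to max and passes its possess capsule, boom, camera transform and behavior tree into inherited variables before running the parent script.
; Tick refreshes the camera transform from a waypoint component, then calls the parent.
; A helper emits noise at the actor's location so AI hearing detects gunshots.
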(event EventTick
  (params (DeltaSeconds :type Float%20%28single-precision%29))
  (bind _camerawaypoint (Variables|Default|GetCameraWaypoint))
  (Variables|Default|SetcameraPos (Math|Transform|MakeTransform (Transformation|GetWorldLocation _camerawaypoint) (Transformation|GetWorldRotation _camerawaypoint)))
  (|CallParentFunction DeltaSeconds))

(fn ConstructionScript
  (bind _camera (Variables|Default|GetCamera))
  (Variables|Default|SetCurrent%20Health (Variables|Default|GetmaxHealth))
  (Variables|Default|SetChildPossessCapsule (Variables|Default|GetPossessCapsule))
  (Variables|Default|SetmainCam (Variables|Default|GetBoomPole))
  (Variables|Default|SetcameraPos (Math|Transform|MakeTransform (Transformation|GetWorldLocation _camera) (Transformation|GetWorldRotation _camera)))
  (Variables|Default|SetBehaviorTree "/Game/Blueprints/Policeman/PoliceBehaviour.PoliceBehaviour")
  (|CallParentFunction))

(fn MakeGunshotNoise
  (bind _self self)
  ;[1 1 1] Makes noise for AI audio detection
  (Class|Actor|MakeNoise 1.0 _self (Transformation|GetActorLocation _self)))