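; Behavior tree service that lets police AI detect the player and switch its blackboard State between Patrol and Attack, starting at enum value 0 on activation.
; While patrolling, each tick box-traces pawns ahead of the policeman; a player hit sets Attack, stores PlayerActor and starts shooting.
; Attack reverts to Patrol when the policeman dies or the player is dead, invisible, missing or beyond SafeDistance.
; Each switch also stops AI movement.
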(event EventReceiveActivation
  (params (OwnerActor :type Actor%20Object%20Reference))
  (Class|BTFunctionLibrary|SetBlackboardValueasEnum (Variables|Default|GetState)))

(event EventTick
  (params (OwnerActor :type Actor%20Object%20Reference) (DeltaSeconds :type Float%20%28single-precision%29))
  (bind _returnvalue (Utilities|Enum|LiteralenumPoliceState "NewEnumerator0"))
  (bind _state (Variables|Default|GetState))
  (bind _playeractor (Variables|Default|GetPlayerActor))
  (bind _returnvalue_2 (Class|BTFunctionLibrary|GetBlackboardValueasEnum _state))
  (bind _returnvalue_3 (Utilities|Enum|ByteToEnumPoliceState _returnvalue_2))
  (bind _asbp_police_ai (Utilities|Casting|CastToBP_PoliceAI OwnerActor))
  (bind _aspoliceman (Utilities|Casting|CastToPoliceman (Pawn|GetControlledPawn _asbp_police_ai)))
  (if (Variables|/Game/Blueprints/EnemyParent/Enemy_Parent.Enemy_Parent_C|Getdead _aspoliceman)
    (switch Utilities|FlowControl|Switch|SwitchonPoliceState _returnvalue_3
      (:NewEnumerator1
        (Class|BTFunctionLibrary|SetBlackboardValueasEnum _state _returnvalue)
        (Class|BTFunctionLibrary|SetBlackboardValueasObject _playeractor (stale _asmy_character))
        (AI|Navigation|StopMovement _asbp_police_ai :!label _label)))
    (else
      (bind _asmy_character (Utilities|Casting|CastToMyCharacter (Game|Player|GetPlayerPawn 0))
        (:then
          (if (or (Variables|/Game/Blueprints/Player/MyCharacter.MyCharacter_C|GetisInvisible _asmy_character) (Variables|/Game/Blueprints/Player/MyCharacter.MyCharacter_C|Getdead _asmy_character))
            (switch Utilities|FlowControl|Switch|SwitchonPoliceState _returnvalue_3 :!label _label_2
              (:NewEnumerator1
                (Class|BTFunctionLibrary|SetBlackboardValueasEnum _state _returnvalue)
                (Class|BTFunctionLibrary|SetBlackboardValueasObject _playeractor _asmy_character)
                (Variables|/Game/Blueprints/Policeman/Policeman.Policeman_C|SetisShooting _aspoliceman false)
                (goto _label)))
            (else
              (switch Utilities|FlowControl|Switch|SwitchonPoliceState (Utilities|Enum|ByteToEnumPoliceState (Class|BTFunctionLibrary|GetBlackboardValueasEnum (Variables|Default|GetState)))
                (:NewEnumerator0
                  (bind _outhits (Class|KismetSystemLibrary|BoxTraceMultiforObjects (+ (Transformation|GetActorLocation _aspoliceman) (* (Math|Vector|GetForwardVector (Transformation|GetActorRotation _aspoliceman)) (.X (Math|Vector|BreakVector (Variables|Default|GetvisionBox))))) (+ (+ (Transformation|GetActorLocation _aspoliceman) (* (Math|Vector|GetForwardVector (Transformation|GetActorRotation _aspoliceman)) (.X (Math|Vector|BreakVector (Variables|Default|GetvisionBox))))) "1.000000,1.000000,1.000000") (Variables|Default|GetvisionBox) (Transformation|GetActorRotation _aspoliceman) (Utilities|Array|MakeArray "ObjectTypeQuery3") false 0 "None" true))
                  (Variables|Default|SethitPlayer false)
                  (bind _array_element (Utilities|Array|ForEachLoopwithBreak _outhits :!label _label_3)
                    (:LoopBody
                      (Variables|Default|SethitPlayer (== (.HitActor (Collision|BreakHitResult _array_element)) _asmy_character))
                      (if (Variables|Default|GethitPlayer)
                        (goto _label_3 Break)))
                    (:Completed
                      (if (Variables|Default|GethitPlayer)
                        (switch Utilities|FlowControl|Switch|SwitchonPoliceState _returnvalue_3
                          (:NewEnumerator0
                            (Class|BTFunctionLibrary|SetBlackboardValueasEnum _state (Utilities|Enum|LiteralenumPoliceState "NewEnumerator1"))
                            (Class|BTFunctionLibrary|SetBlackboardValueasObject _playeractor _asmy_character)
                            (Variables|/Game/Blueprints/Policeman/Policeman.Policeman_C|SetisShooting _aspoliceman true)
                            (goto _label)))
                        (else
                          (goto _label_2))))))
                (:NewEnumerator1
                  (if (> (Math|Float|Absolute(Float) (Math|Vector|VectorLength (- (Transformation|GetActorLocation _asmy_character) (Transformation|GetActorLocation _aspoliceman)))) (Variables|Default|GetsafeDistance))
                    (goto _label_2)))))))
        (:CastFailed
          (goto _label_2))))))