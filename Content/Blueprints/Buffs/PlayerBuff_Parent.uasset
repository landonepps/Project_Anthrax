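; PlayerBuff_Parent is a timed area actor that buffs any MyCharacter inside its sphere.
; Overlap begin and end call ApplyBuff and RemoveBuff on the character with a hard-coded enum value, leaving the Buff variable unused.
; The construction script sizes the sphere from Radius.
; Tick counts DurationTime down through HandleDurationTime and destroys the actor when it runs out.
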(event OnComponentEndOverlap(Sphere)
  (params (OtherActor :type Actor%20Object%20Reference) (OtherComp :type Primitive%20Component%20Object%20Reference) (OtherBodyIndex :type Integer))
  (bind _asmy_character (Utilities|Casting|CastToMyCharacter OtherActor))
  (Default|RemoveBuff _asmy_character "NewEnumerator1"))

(event OnComponentBeginOverlap(Sphere)
  (params (OtherActor :type Actor%20Object%20Reference) (OtherComp :type Primitive%20Component%20Object%20Reference) (OtherBodyIndex :type Integer) (bFromSweep :type Boolean) (SweepResult :type Hit%20Result%20Structure%20%28by%20ref%29))
  (bind _asmy_character (Utilities|Casting|CastToMyCharacter OtherActor))
  (Default|ApplyBuff _asmy_character "NewEnumerator1"))

(event EventBeginPlay)

(event EventActorBeginOverlap
  (params (OtherActor :type Actor%20Object%20Reference)))

(event EventTick
  (params (DeltaSeconds :type Float%20%28single-precision%29))
  (CallFunction|HandleDurationTime DeltaSeconds))

(fn ConstructionScript
  (Components|Sphere|SetSphereRadius (Variables|Default|GetSphere) (Variables|Default|GetRadius) true))

(fn HandleDurationTime
  (params (DeltaTime :type Float%20%28single-precision%29 :default 0.0))
  (bind _output_get (Variables|Default|SetdurationTime (- (Variables|Default|GetdurationTime) DeltaTime)))
  (if (<= _output_get 0.0)
    (Actor|DestroyActor)))