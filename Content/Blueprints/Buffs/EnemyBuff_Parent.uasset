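; EnemyBuff_Parent is a timed area actor that, judging by its name, serves as the base for enemy buff zones.
; Its sphere, sized from Radius at construction, applies Buff to any Enemy_Parent entering it and removes Buff when that enemy leaves.
; Tick counts DurationTime down, destroying the actor when it runs out, and slowly spins the decal.
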(event OnComponentEndOverlap(Sphere)
  (params (OtherActor :type Actor%20Object%20Reference) (OtherComp :type Primitive%20Component%20Object%20Reference) (OtherBodyIndex :type Integer))
  (bind _asenemy_parent (Utilities|Casting|CastToEnemy_Parent OtherActor))
  (Default|RemoveBuff _asenemy_parent (Variables|Default|GetBuff)))

(event OnComponentBeginOverlap(Sphere)
  (params (OtherActor :type Actor%20Object%20Reference) (OtherComp :type Primitive%20Component%20Object%20Reference) (OtherBodyIndex :type Integer) (bFromSweep :type Boolean) (SweepResult :type Hit%20Result%20Structure%20%28by%20ref%29))
  (bind _asenemy_parent (Utilities|Casting|CastToEnemy_Parent OtherActor))
  (Default|ApplyBuff _asenemy_parent (Variables|Default|GetBuff)))

(event EventBeginPlay)

(event EventActorBeginOverlap
  (params (OtherActor :type Actor%20Object%20Reference)))

(event EventTick
  (params (DeltaSeconds :type Float%20%28single-precision%29))
  (CallFunction|HandleDurationTime DeltaSeconds)
  (CallFunction|SpinDecal DeltaSeconds))

(fn ConstructionScript
  (Components|Sphere|SetSphereRadius (Variables|Default|GetSphere) (Variables|Default|GetRadius) true))

(fn HandleDurationTime
  (params (DeltaTime :type Float%20%28single-precision%29 :default 0.0))
  (bind _output_get (Variables|Default|SetdurationTime (- (Variables|Default|GetdurationTime) DeltaTime)))
  (if (<= _output_get 0.0)
    (Actor|DestroyActor)))

(fn SpinDecal
  (params (DeltaTime :type Float%20%28single-precision%29 :default 0.0))
  (bind _output_get (Variables|Default|SetSpin (+ (Variables|Default|GetSpin) (* DeltaTime 1e+01))))
  (Transformation|SetRelativeRotation (Variables|Default|GetDecal) (Class|KismetMathLibrary|MakeRot 9e+01 _output_get 0.0) false))