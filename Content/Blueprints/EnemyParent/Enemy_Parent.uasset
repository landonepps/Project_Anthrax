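; Base enemy character that takes damage, becomes stunned at or below an execution-threshold health, and dies into a ragdoll.
; Tick toggles a component's visibility with the stun state, turns the health bar toward the player camera, updates its fill and scales walk speed.
; Damage plays grunt or death sounds and reports kills to MyCharacter.
; Player collisions fire a touched dispatcher and push the hit actor away, much farther during a dodge.
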(event EventTick
  (params (DeltaSeconds :type Float%20%28single-precision%29))
  (bind _healthbar (Variables|Default|GethealthBar))
  (bind _output_get (Variables|Default|SetStunned (<= (Variables|Default|Gethealth) (Variables|Default|GetExecutionThreshold))))
  (Rendering|SetVisibility _output_get false)
  ;[1 1 1] Display Health
  (if (Variables|Default|GetisDead)
    (Utilities|FlowControl|DoOnce false
      (:Completed
        (Components|DestroyComponent)
        (Components|DestroyComponent)))
    (else
      (bind _asmy_character (Utilities|Casting|CastToMyCharacter (Game|GetPlayerCharacter 0)))
      ;;[1 1 1] not quite right
      (Transformation|SetWorldRotation _healthbar (Class|KismetMathLibrary|MakeRot 0.0 (- (.Yaw (Class|KismetMathLibrary|BreakRot (Math|Rotator|FindLookatRotation (Transformation|GetWorldLocation _healthbar) (Transformation|GetWorldLocation (Variables|/Script/Project_Anthrax.Project_AnthraxCharacter|GetFollowCamera _asmy_character))))) 9e+01) 9e+01) false) ; this rotation doesn't quite work
      (bind _asenemy_health (Utilities|Casting|CastToEnemyHealth (UserInterface|GetUserWidgetObject (Variables|Default|GethealthBar))))
      (Variables|/Game/UserInterface/EnemyHealth.EnemyHealth_C|SethealthPercentage _asenemy_health (/ (Variables|Default|Gethealth) (Variables|Default|GetmaxHealth)))
      ;[1 1 1] Movement Speed
      (Variables|/Script/Engine.CharacterMovementComponent|SetMaxWalkSpeed (Variables|Character|GetCharacterMovement) (* (Variables|Default|GetspeedScaleFactor) (Variables|Default|GetmaxSpeed))))))

(event EventHit
  (params (MyComp :type Primitive%20Component%20Object%20Reference) (Other :type Actor%20Object%20Reference) (OtherComp :type Primitive%20Component%20Object%20Reference) (bSelfMoved :type Boolean) (HitLocation :type Vector :default "0, 0, 0") (HitNormal :type Vector :default "0, 0, 0") (NormalImpulse :type Vector :default "0, 0, 0") (Hit :type Hit%20Result%20Structure%20%28by%20ref%29))
  (bind _hitactor (Collision|BreakHitResult Hit))
  (bind _returnvalue (Game|Player|GetPlayerPawn 0))
  (bind _returnvalue_2 (Transformation|GetActorLocation _returnvalue))
  (bind _returnvalue_3 (Transformation|GetActorLocation _hitactor))
  (bind _returnvalue_4 (Math|Rotator|FindLookatRotation _returnvalue_2 _returnvalue_3))
  (bind _returnvalue_5 (Math|Rotator|GetRotationXVector _returnvalue_4))
  ;[1 1 1] Reacte to player collision
  (bind _asmy_character (Utilities|Casting|CastToMyCharacter _returnvalue))
  (if (== _asmy_character Other)
    (Default|CallEnemyTouchedDispatcher)
    (if (Variables|/Game/Blueprints/Player/MyCharacter.MyCharacter_C|GetisDodging _asmy_character)
      ;;[1 1 1] Move to New Location
      (Transformation|SetActorLocation _hitactor (+ _returnvalue_3 (* _returnvalue_5 2e+02)) true)
      (else
        (Transformation|SetActorLocation _hitactor (+ (* _returnvalue_5 5.0) _returnvalue_3) true)))))

(event EventTakeDamage
  (params (attackDamage :type Float%20%28single-precision%29))
  (bind _mesh (Variables|Character|GetMesh))
  ;[1 1 1] Take Damage
  (if (not (Variables|Default|GetisDead))
    (Variables|UserOptions|Basic|SetHealth (- (Variables|Default|GetHealth) attackDamage))
    (Class|GameplayStatics|PlaySoundAttached "/Game/Audio/DamageAudio/low_grunt1.low_grunt1" _mesh)
    (if (<= (Variables|Default|GetHealth) 0.0)
      (Variables|Default|SetisDead true)
      (Class|GameplayStatics|PlaySoundAttached "/Game/Audio/DamageAudio/male_death1.male_death1" _mesh)
      (Physics|SetSimulatePhysics (Variables|Character|GetMesh) true)
      (Collision|SetCollisionEnabled (Variables|Collision|GetCapsuleComponent) "NoCollision")
      (Components|DestroyComponent)
      (bind _asmy_character (Utilities|Casting|CastToMyCharacter (Game|GetPlayerCharacter 0)))
      (Default|EnemyKilled _asmy_character self))))

(fn ConstructionScript)

(fn GetHealth
  ;[1 1 1] Returns Health
  (return (Variables|Default|Gethealth)))