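; Base possessable pawn that the player character can take over, hop between and leave, with GetMesh left empty, presumably for children.
; A capsule overlap selects the neighbour nearest a fixed screen point and highlights it via custom depth.
; Possession saves the camera transform and interpolates MainCam to CameraPos for a smooth handoff.
; Unpossess box-checks the space ahead, then restores the character there if clear and no object is selected.
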(event OnComponentEndOverlap(ChildPossessCapsule)
  (params (OtherActor :type Actor%20Object%20Reference) (OtherComp :type Primitive%20Component%20Object%20Reference) (OtherBodyIndex :type Integer))
  ;[1 1 1] Disable Highlight on Objects
  (if (== self (Pawn|GetControlledPawn (Game|GetPlayerController 0)))
    (bind _aspossessable_object_p (Utilities|Casting|CastToPossessableObject_P OtherActor))
    (if (== _aspossessable_object_p (Variables|Default|GetSelected%20Possession%20Object))
      (Variables|Default|SetSelected%20Possession%20Object 0))
    (CallFunction|SetHighlightActive _aspossessable_object_p false)))

(event OnComponentBeginOverlap(ChildPossessCapsule)
  (params (OtherActor :type Actor%20Object%20Reference) (OtherComp :type Primitive%20Component%20Object%20Reference) (OtherBodyIndex :type Integer) (bFromSweep :type Boolean) (SweepResult :type Hit%20Result%20Structure%20%28by%20ref%29))
  (bind _childpossesscapsule (Variables|Default|GetChildPossessCapsule))
  ;[1 1 1] Possession Logic With Highlight
  (Utilities|Casting|CastToPossessableObject_P OtherActor)
  (if (Utilities|IsValid _childpossesscapsule)
    (bind (_outactors _returnvalue) (Class|KismetSystemLibrary|ComponentOverlapActorsNEW _childpossesscapsule (Transformation|GetWorldTransform) (Utilities|Array|MakeArray "ObjectTypeQuery1") "PossessableObject_P_C"))
    (Variables|Default|SetpossessableObjectDistFromScreenCenter 1000000)
    (for _array_element _outactors
      ;;[1 1 1] Loop over all Possessable Objects colliding with PossessCapsule and determine center-most object
      (if (not (== _array_element self))
        (bind _aspossessable_object_p (Utilities|Casting|CastToPossessableObject_P _array_element))
        (CallFunction|SetHighlightActive _aspossessable_object_p false)
        (if (< (Math|Vector2D|Vector2DLength (- (.ScreenLocation (Class|PlayerController|ProjectWorldLocationtoScreen (Game|GetPlayerController 0) (Transformation|GetActorLocation _array_element))) "(X=700.000000,Y=700.000000)")) (Math|Conversions|ToFloat(Integer) (Variables|Default|GetpossessableObjectDistFromScreenCenter)))
          (Variables|Default|SetpossessableObjectDistFromScreenCenter (Math|Float|Floor (Math|Vector2D|Vector2DLength (- (.ScreenLocation (Class|PlayerController|ProjectWorldLocationtoScreen (Game|GetPlayerController 0) (Transformation|GetActorLocation _array_element))) "(X=700.000000,Y=700.000000)"))))
          (Variables|Default|SetSelected%20Possession%20Object _array_element))))
    (if _returnvalue
      (bind _aspossessable_object_p_2 (Utilities|Casting|CastToPossessableObject_P (Variables|Default|GetSelected%20Possession%20Object)))
      (CallFunction|SetHighlightActive _aspossessable_object_p_2 true))
    (else
      (Development|PrintString 0 "ERROR: PossessCapsule not initialized"))))

(event Custom|Check%20Possession%20Logic%20With%20Highlight
  (bind _childpossesscapsule (Variables|Default|GetChildPossessCapsule))
  ;[1 1 1] Possession Logic With Highlight
  (if (Utilities|IsValid _childpossesscapsule)
    (bind (_outactors _returnvalue) (Class|KismetSystemLibrary|ComponentOverlapActorsNEW _childpossesscapsule (Transformation|GetWorldTransform) (Utilities|Array|MakeArray "ObjectTypeQuery1") "PossessableObject_P_C"))
    (Variables|Default|SetpossessableObjectDistFromScreenCenter 1000000)
    (for _array_element _outactors
      ;;[1 1 1] Loop over all Possessable Objects colliding with PossessCapsule and determine center-most object
      (if (not (== _array_element self))
        (bind _aspossessable_object_p (Utilities|Casting|CastToPossessableObject_P _array_element))
        (CallFunction|SetHighlightActive _aspossessable_object_p false)
        (if (< (Math|Vector2D|Vector2DLength (- (.ScreenLocation (Class|PlayerController|ProjectWorldLocationtoScreen (Game|GetPlayerController 0) (Transformation|GetActorLocation _array_element))) "(X=700.000000,Y=700.000000)")) (Math|Conversions|ToFloat(Integer) (Variables|Default|GetpossessableObjectDistFromScreenCenter)))
          (Variables|Default|SetpossessableObjectDistFromScreenCenter (Math|Float|Floor (Math|Vector2D|Vector2DLength (- (.ScreenLocation (Class|PlayerController|ProjectWorldLocationtoScreen (Game|GetPlayerController 0) (Transformation|GetActorLocation _array_element))) "(X=700.000000,Y=700.000000)"))))
          (Variables|Default|SetSelected%20Possession%20Object _array_element))))
    (if _returnvalue
      (bind _aspossessable_object_p_2 (Utilities|Casting|CastToPossessableObject_P (Variables|Default|GetSelected%20Possession%20Object)))
      (CallFunction|SetHighlightActive _aspossessable_object_p_2 true))
    (else
      (Development|PrintString 0 "ERROR: PossessCapsule not initialized"))))

(event Custom|Possession%20Highlight
  ;[1 1 1] Possession Highlight
  (bind _asmesh_component (Utilities|Casting|CastToMeshComponent (CallFunction|GetMesh)))
  (Rendering|SetRenderCustomDepth _asmesh_component (Variables|Default|GethighlightActive)))

(event Custom|Transition%20Camera
  (bind _maincam (Variables|Default|GetmainCam))
  ;[1 1 1] Transition Camera smoothly when possessing
  (Transformation|SetWorldLocation _maincam (Math|Interpolation|VInterpTo (Transformation|GetWorldLocation _maincam) (.Location (Math|Transform|BreakTransform (Variables|Default|GetcameraPos))) (Utilities|Time|GetWorldDeltaSeconds) (Variables|Default|GetcameraTransitionSpeed)) false))

(event EventTick
  (params (DeltaSeconds :type Float%20%28single-precision%29))
  (CallFunction|PossessionHighlight)
  (CallFunction|TransitionCamera))

(event EventEnterPossession
  (params (playerPawn :type Pawn%20Object%20Reference))
  ;[1 1 1] Enter Possession
  (Variables|Default|SetplayerPawn playerPawn)
  (bind _asmy_character (Utilities|Casting|CastToMyCharacter playerPawn))
  (Default|EnableCharacter _asmy_character false)
  (Collision|SetCollisionEnabled "QueryAndPhysics")
  (CallFunction|CheckPossessionLogicwithHighlight)
  (CallFunction|EnterPossession))

(event EventBeginPlay
  ;[1 1 1] Startup logic to ensure that all variables are set
  (if (Utilities|IsValid (Variables|Default|GetChildPossessCapsule))
    (if (Utilities|IsValid (Variables|Default|GetmainCam))
      (if (Math|Vector|NotEqual(Vector) (.Location (Math|Transform|BreakTransform (Variables|Default|GetcameraPos))) "0, 0, 0" 0.0001)
        (Collision|SetCollisionEnabled (Variables|Default|GetChildPossessCapsule) "NoCollision")
        (else
          (Development|PrintString 0 (Utilities|String|Append (Utilities|String|Append (Utilities|String|MakeLiteralString "ERROR: ") (Utilities|GetDisplayName self)) "has no CameraDefaultPos"))))
      (else
        (Development|PrintString 0 (Utilities|String|Append (Utilities|String|Append (Utilities|String|MakeLiteralString "ERROR: ") (Utilities|GetDisplayName self)) "has no MainCam"))))
    (else
      (Development|PrintString 0 (Utilities|String|Append (Utilities|String|Append (Utilities|String|MakeLiteralString "ERROR: ") (Utilities|GetDisplayName self)) "has no ChildPossessCapsule")))))

(event Input|ActionEvents|InputActionPossess
  (bind _selected_possession_object (Variables|Default|GetSelected%20Possession%20Object))
  ;[1 1 1] Possess selected object
  (:Pressed
    (if (Utilities|IsValid _selected_possession_object)
      (Class|PossessableI|EnterPossession(Message) _selected_possession_object (Variables|Default|GetplayerPawn)))))

(event Input|ActionEvents|InputActionUnpossess
  (bind _returnvalue (Game|GetPlayerCameraManager 0))
  (bind _mesh (CallFunction|GetMesh))
  (bind _returnvalue_2 (Camera|GetCameraRotation _returnvalue))
  (bind _returnvalue_3 (Transformation|GetWorldLocation _mesh))
  (bind _yaw (Class|KismetMathLibrary|BreakRot _returnvalue_2))
  (bind _returnvalue_4 (+ _returnvalue_3 "0,0.000000,100.000000"))
  (bind _returnvalue_5 (Class|KismetMathLibrary|MakeRot 0.0 _yaw 0.0))
  (bind _returnvalue_6 (Math|Vector|GetForwardVector _returnvalue_5))
  (bind _returnvalue_7 (* _returnvalue_6 1.5e+02))
  (bind _returnvalue_8 (+ _returnvalue_4 _returnvalue_7))
  ;[1 1 1] Exit Possession
  (:Pressed
    (bind _returnvalue_9 (Class|KismetSystemLibrary|BoxOverlapActorsNEW 0 _returnvalue_8 "30.000000,30.000000,60.000000" (Utilities|Array|MakeArray "ObjectTypeQuery1")))
    (if _returnvalue_9
      (CallFunction|CheckPossessionLogicwithHighlight)
      (if (not (Utilities|IsValid (Variables|Default|GetSelected%20Possession%20Object)))
        (Class|GameplayStatics|PlaySoundAttached "/Game/Audio/PlayerAudio/swoosh.swoosh" (CallFunction|GetMesh)))
      (else
        (Transformation|SetActorLocationAndRotation (Variables|Default|GetplayerPawn) _returnvalue_8 (Class|KismetMathLibrary|MakeRot 0.0 (.Yaw (Class|KismetMathLibrary|BreakRot _returnvalue_2)) 0.0))
        (Collision|SetCollisionEnabled "NoCollision")
        (CallFunction|CheckPossessionLogicwithHighlight)
        (if (not (Utilities|IsValid (Variables|Default|GetSelected%20Possession%20Object)))
          (CallFunction|ExitPossession))))))

(event Input|ActionEvents|InputActionGoInvisible
  (bind _playerpawn (Variables|Default|GetplayerPawn))
  (:Pressed
    (bind _asmy_character (Utilities|Casting|CastToMyCharacter _playerpawn)
      (:then
        (Variables|/Game/Blueprints/Player/MyCharacter.MyCharacter_C|SetisInvisible _asmy_character true)
        (Default|InvisibilityChanged _asmy_character :!label _label))
      (:CastFailed
        (Development|PrintString 0 :!label _label_2))))
  (:Released
    (bind _asmy_character_2 (Utilities|Casting|CastToMyCharacter _playerpawn)
      (:then
        (Variables|/Game/Blueprints/Player/MyCharacter.MyCharacter_C|SetisInvisible _asmy_character_2 false)
        (goto _label))
      (:CastFailed
        (goto _label_2)))))

(event Input|AxisEvents|InputAxisTurn
  (params (AxisValue :type Float%20%28single-precision%29))
  ;[1 1 1] Camera Controls
  (Transformation|AddWorldRotation (Variables|Default|GetmainCam) (Class|KismetMathLibrary|MakeRot 0.0 AxisValue 0.0) false))

(event Input|AxisEvents|InputAxisLookUp
  (params (AxisValue :type Float%20%28single-precision%29))
  ;[1 1 1] Camera Controls
  (Transformation|AddLocalRotation (Variables|Default|GetmainCam) (Class|KismetMathLibrary|MakeRot (* AxisValue -1.0) 0.0 0.0) false))

(fn ConstructionScript)

(fn EnterPossession
  (bind _returnvalue (Game|GetPlayerCameraManager 0))
  (if (Utilities|IsValid (Variables|Default|GetSelected%20Possession%20Object))
    (bind _aspossessable_object_p (Utilities|Casting|CastToPossessableObject_P (Variables|Default|GetSelected%20Possession%20Object)))
    (CallFunction|SetHighlightActive _aspossessable_object_p false)
    (Variables|Default|SetSelected%20Possession%20Object 0))
  (bind _asmy_character (Utilities|Casting|CastToMyCharacter (Variables|Default|GetplayerPawn)))
  (Default|SetIsPossessing _asmy_character true)
  (Variables|Default|SethighlightActive false)
  ;[1 1 1] Possess the object and set camera for transition
  (Variables|Default|SettransitionCam (Math|Transform|MakeTransform (Camera|GetCameraLocation _returnvalue) (Camera|GetCameraRotation _returnvalue)))
  (Pawn|Possess (Game|GetPlayerController 0) self)
  (Transformation|SetWorldLocationAndRotation (Variables|Default|GetmainCam) (.Location (Math|Transform|BreakTransform (Variables|Default|GettransitionCam))) (.Rotation (Math|Transform|BreakTransform (Variables|Default|GettransitionCam))) false))

(fn ExitPossession
  (bind _playerpawn (Variables|Default|GetplayerPawn))
  (bind _maincam (Variables|Default|GetmainCam))
  (Variables|Default|SethighlightActive false)
  (if (Utilities|IsValid (Variables|Default|GetSelected%20Possession%20Object))
    (bind _aspossessable_object_p (Utilities|Casting|CastToPossessableObject_P (Variables|Default|GetSelected%20Possession%20Object)))
    (CallFunction|SetHighlightActive _aspossessable_object_p false)
    (Variables|Default|SetSelected%20Possession%20Object 0))
  (bind _asmy_character (Utilities|Casting|CastToMyCharacter _playerpawn))
  (Default|EnableCharacter _asmy_character true)
  (Default|SetIsPossessing _asmy_character false)
  (Variables|Default|SettransitionCam (Math|Transform|MakeTransform (Transformation|GetWorldLocation _maincam) (Transformation|GetWorldRotation _maincam)))
  (Pawn|Possess (Game|GetPlayerController 0) _playerpawn)
  (Default|SetCamera _asmy_character (Variables|Default|GettransitionCam)))

(fn GetMesh
  (return 0))

(fn SetHighlightActive
  (params (active :type Boolean))
  (Variables|Default|SethighlightActive active))