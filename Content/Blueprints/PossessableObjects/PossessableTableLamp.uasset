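; A possessable table lamp, built as a child of a parent possessable-object Blueprint.
; Its construction script fills inherited-style references with its own possess capsule and boom pole, and stores Camera10's world location and rotation as the camera transform, before running the parent script.
; GetMesh returns the lamp's static mesh, and the event graph holds only an unconnected debug print of the highlight state.
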(fn ConstructionScript
  (bind _camera1_0 (Variables|Default|GetCamera1_0))
  (Variables|Default|SetChildPossessCapsule (Variables|Default|GetPossessCapsule))
  (Variables|Default|SetmainCam (Variables|Default|GetBoomPole))
  (Variables|Default|SetcameraPos (Math|Transform|MakeTransform (Transformation|GetWorldLocation _camera1_0) (Transformation|GetWorldRotation _camera1_0)))
  (|CallParentFunction))

(fn GetMesh
  (return (Variables|Default|GetStaticMesh1)))