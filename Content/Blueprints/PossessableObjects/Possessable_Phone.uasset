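; Possessable phone that rings when activated, playing an attached sound and emitting noise at its location.
; An Activated flag blocks retriggering until the ring-time delay ends.
; The construction script passes its capsule, boom pole and camera transform into inherited variables before running the parent script, and GetMesh returns the phone's static mesh.
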(event EventActivatePossessable
  (bind _self self)
  ;[1 1 1] Handle Possessable
  (if (not (Variables|Default|Getactivated))
    (Variables|Default|Setactivated true)
    (Class|GameplayStatics|PlaySoundAttached "/Game/Audio/ObjectAudio/Ringing_Phone_Cue.Ringing_Phone_Cue" (Variables|Default|GetStaticMesh1))
    (Class|PawnNoiseEmitterComponent|MakeNoise _self (Variables|Default|GetphoneLoudness) (Transformation|GetActorLocation _self))
    (Utilities|FlowControl|Delay (Variables|Default|GetPhoneRingTime))
    (Variables|Default|Setactivated false)))

(fn ConstructionScript
  (bind _camera1_0 (Variables|Default|GetCamera1_0))
  (Variables|Default|SetChildPossessCapsule (Variables|Default|GetPossessCapsule))
  (Variables|Default|SetmainCam (Variables|Default|GetBoomPole))
  (Variables|Default|SetcameraPos (Math|Transform|MakeTransform (Transformation|GetWorldLocation _camera1_0) (Transformation|GetWorldRotation _camera1_0)))
  (|CallParentFunction))

(fn GetMesh
  (return (Variables|Default|GetStaticMesh1)))