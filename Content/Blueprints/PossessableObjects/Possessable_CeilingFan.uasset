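; A possessable ceiling fan, built on a parent possessable class, that can be switched to spin.
; Activating it toggles a flag, and while that is set each Tick adds a fixed rotation to the fan mesh, so speed depends on frame rate.
; The construction script hands its possess capsule, boom pole and camera transform to inherited variables before running the parent's script.
; GetMesh returns the fan mesh.
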(event Custom|HandleActivated
  (bind _staticmesh1 (Variables|Default|GetStaticMesh1))
  (if (Variables|Default|Getactivated)
    (Transformation|SetWorldRotation _staticmesh1 (Math|Rotator|CombineRotators (Transformation|GetWorldRotation _staticmesh1) "0,10.000000, 0") false)))

(event EventTick
  (params (DeltaSeconds :type Float%20%28single-precision%29))
  ;[1 1 1] Event Tick
  (|CallParentFunction DeltaSeconds)
  (CallFunction|HandleActivated))

(event EventActivatePossessable
  ;[1 1 1] Activate Possessable
  (Variables|Default|Setactivated (not (Variables|Default|Getactivated))))

(fn ConstructionScript
  (bind _camera1_0 (Variables|Default|GetCamera1_0))
  (Variables|Default|SetChildPossessCapsule (Variables|Default|GetPossessCapsule))
  (Variables|Default|SetmainCam (Variables|Default|GetBoomPole))
  (Variables|Default|SetcameraPos (Math|Transform|MakeTransform (Transformation|GetWorldLocation _camera1_0) (Transformation|GetWorldRotation _camera1_0)))
  (|CallParentFunction))

(fn GetMesh
  (return (Variables|Default|GetStaticMesh1)))