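; Door actor that swings open when a Player-tagged actor enters its Trigger and closes when that actor leaves, unless Locked.
; The RotateDoor timeline adds yaw to the rotation captured on entry, playing forward to open and in reverse to close.
; Open flips only when the timeline finishes, so leaving mid-swing does not start closing.
; LockDoor and UnlockDoor set and return the Locked flag.
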(event OnComponentEndOverlap(Trigger)
  (params (OtherActor :type Actor%20Object%20Reference) (OtherComp :type Primitive%20Component%20Object%20Reference) (OtherBodyIndex :type Integer))
  (bind _doorrotation (Variables|Default|GetdoorRotation))
  (bind (_pitch _yaw _roll) (Class|KismetMathLibrary|BreakRot _doorrotation))
  (if (Variables|Default|GetOpen)
    (if (not (Variables|Default|GetLocked))
      (if (Actor|ActorHasTag OtherActor "Player")
        (bind _door_rotation (Timeline|Rotate%20Door Reverse)
          (:Update
            (Transformation|SetActorRotation (Class|KismetMathLibrary|MakeRot _pitch (+ _door_rotation _yaw) _roll)))
          (:Finished
            (Variables|Default|SetOpen (not (Variables|Default|GetOpen)))))))))

(event OnComponentBeginOverlap(Trigger)
  (params (OtherActor :type Actor%20Object%20Reference) (OtherComp :type Primitive%20Component%20Object%20Reference) (OtherBodyIndex :type Integer) (bFromSweep :type Boolean) (SweepResult :type Hit%20Result%20Structure%20%28by%20ref%29))
  (if (not (Variables|Default|GetOpen))
    (Variables|Default|SetdoorRotation (Transformation|GetActorRotation))
    (if (not (Variables|Default|GetLocked))
      (if (Actor|ActorHasTag OtherActor "Player")
        (bind _door_rotation (Timeline|Rotate%20Door Play)
          (:Update
            (Transformation|SetActorRotation (Class|KismetMathLibrary|MakeRot (.Pitch (Class|KismetMathLibrary|BreakRot (Variables|Default|GetdoorRotation))) (+ _door_rotation (.Yaw (Class|KismetMathLibrary|BreakRot (Variables|Default|GetdoorRotation)))) (.Roll (Class|KismetMathLibrary|BreakRot (Variables|Default|GetdoorRotation))))))
          (:Finished
            (Variables|Default|SetOpen (not (Variables|Default|GetOpen)))))))))

(fn ConstructionScript)

(fn LockDoor
  (Variables|Default|SetLocked true)
  (return (Variables|Default|GetLocked)))

(fn UnlockDoor
  (Variables|Default|SetLocked false)
  (return (Variables|Default|GetLocked)))