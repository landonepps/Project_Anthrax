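; Behavior tree node for the dummy enemy that flags whether the player counts as found.
; Each tick it casts the player pawn to MyCharacter and sets the PlayerFoundKey blackboard bool true only when the character is neither possessing nor invisible.
; It performs no distance or sight check.
; Debug prints show the possession state, or a placeholder message if the cast fails.
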(event EventTick
  (params (OwnerActor :type Actor%20Object%20Reference) (DeltaSeconds :type Float%20%28single-precision%29))
  (bind _asmy_character (Utilities|Casting|CastToMyCharacter (Game|Player|GetPlayerPawn 0))
    (:then
      (Development|PrintString (Utilities|String|ToString(Boolean) (Variables|/Game/Blueprints/MyCharacter.MyCharacter_C|GetisPossessing _asmy_character))))
    (:CastFailed
      (Development|PrintString "Hello")))
  (Class|BTFunctionLibrary|SetBlackboardValueasBool (Variables|Default|GetplayerFoundKey) (not (or (Variables|/Game/Blueprints/MyCharacter.MyCharacter_C|GetisPossessing _asmy_character) (Variables|/Game/Blueprints/MyCharacter.MyCharacter_C|GetisInvisible _asmy_character)))))