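; Player character Blueprint with three abilities: slashing enemies, turning translucent for invisibility and possessing objects.
; Slashing enables socket-attached hand collision, with left-hand overlaps sending attack messages to DummyEnemy.
; Invisibility swaps to a dynamic translucent material whose opacity follows a timeline.
; Each tick highlights the capsule-overlapped PossessableObject_P nearest a hardcoded screen point, and the Possess input sends it an enter-possession message.
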(event OnComponentBeginOverlap(HandCollision_L)
  (params (OtherActor :type Actor%20Object%20Reference) (OtherComp :type Primitive%20Component%20Object%20Reference) (OtherBodyIndex :type Integer) (bFromSweep :type Boolean) (SweepResult :type Hit%20Result%20Structure%20%28by%20ref%29))
  (if (Variables|Default|GetisSlashing)
    (bind _asdummy_enemy (Utilities|Casting|CastToDummyEnemy OtherActor))
    (Class|PlayerEnemyI|PlayerAttack(Message) _asdummy_enemy (Game|Player|GetPlayerPawn 0))))

(event OnComponentEndOverlap(PossessCapsule)
  (params (OtherActor :type Actor%20Object%20Reference) (OtherComp :type Primitive%20Component%20Object%20Reference) (OtherBodyIndex :type Integer))
  ;[1 1 1] Disable Highlight on Objects
  (bind _aspossessable_object_p (Utilities|Casting|CastToPossessableObject_P OtherActor))
  (Default|SetHighlightActive _aspossessable_object_p false))

(event Custom|CheckPossession
  ;[1 1 1] Possession Logic With Highlight
  (bind (_outactors _returnvalue) (Class|KismetSystemLibrary|ComponentOverlapActorsNEW (Variables|Default|GetPossessCapsule) (Transformation|GetWorldTransform) (Utilities|Array|MakeArray "ObjectTypeQuery1") "/Game/Blueprints/PossessableObjects/PossessableObject_P.PossessableObject_P_C"))
  (Variables|Default|SetpossessableObjectDistFromScreenCenter 1000000)
  (for _array_element _outactors
    ;;[1 1 1] Loop over all Possessable Objects colliding with PossessCapsule and determine center-most object
    (bind _aspossessable_object_p (Utilities|Casting|CastToPossessableObject_P _array_element))
    (Default|SetHighlightActive _aspossessable_object_p false)
    (if (< (Math|Vector2D|Vector2DLength (- (.ScreenLocation (Class|PlayerController|ProjectWorldLocationtoScreen (Game|GetPlayerController 0) (Transformation|GetActorLocation _array_element))) "(X=700.000000,Y=700.000000)")) (Math|Conversions|ToFloat(Integer) (Variables|Default|GetpossessableObjectDistFromScreenCenter)))
      (Variables|Default|SetpossessableObjectDistFromScreenCenter (Math|Float|Floor (Math|Vector2D|Vector2DLength (- (.ScreenLocation (Class|PlayerController|ProjectWorldLocationtoScreen (Game|GetPlayerController 0) (Transformation|GetActorLocation _array_element))) "(X=700.000000,Y=700.000000)"))))
      (Variables|Default|SetSelected%20Possession%20Object _array_element)))
  (if _returnvalue
    (bind _aspossessable_object_p_2 (Utilities|Casting|CastToPossessableObject_P (Variables|Default|GetSelected%20Possession%20Object)))
    (Default|SetHighlightActive _aspossessable_object_p_2 true)))

(event Custom|Tried%20Invisibility%20Event
  ;[1 1 1] Invisbility Logic
)

(event Custom|Tried%20Possession%20Event
  ;[1 1 1] Possess selected object
)

(event EventTick
  (params (DeltaSeconds :type Float%20%28single-precision%29))
  (CallFunction|CheckPossession))

(event Input|ActionEvents|InputActionPossess
  ;[1 1 1] Possess selected object
  (:Pressed
    (if (< (Variables|Default|GetpossessableObjectDistFromScreenCenter) 1000000)
      (Class|PossessableI|EnterPossession(Message) (Variables|Default|GetSelected%20Possession%20Object) (Game|Player|GetPlayerPawn 0))
      (EventDispatchers|BindEventtoTriedPossession (delegate Custom|Tried%20Possession%20Event))
      (Default|CallTriedPossession))))

(event Input|GamepadEvents|GamepadRightTrigger
  ;[1 1 1] Slashing attack
  (:Pressed
    (Variables|Default|SetisSlashing true)
    (Collision|SetCollisionEnabled (Variables|Default|GetHandCollision_L) "QueryAndPhysics"))
  (:Released
    (Variables|Default|SetisSlashing false)
    (Collision|SetCollisionEnabled (Variables|Default|GetHandCollision_R) "NoCollision")))

(event Input|MouseEvents|LeftMouseButton
  ;[1 1 1] Slashing attack
  (:Pressed
    (Variables|Default|SetisSlashing true)
    (Collision|SetCollisionEnabled (Variables|Default|GetHandCollision_L) "QueryAndPhysics"))
  (:Released
    (Variables|Default|SetisSlashing false)
    (Collision|SetCollisionEnabled (Variables|Default|GetHandCollision_R) "NoCollision")))

(event Input|GamepadEvents|GamepadLeftTrigger
  ;[1 1 1] Invisbility Logic
  (:Pressed
    (Variables|Default|SetisInvisible true)
    (Rendering|Material|SetMaterial 0 (Variables|Default|GettranslucentMaterial))
    (EventDispatchers|BindEventtoTriedInvisibility (delegate Custom|Tried%20Invisibility%20Event))
    (Default|CallTriedInvisibility)
    (bind _transition (Timeline|Opacity%20Change Play)
      (:Update
        (Rendering|Material|SetScalarParameterValue (Variables|Default|GettranslucentMaterial) "Opacity" _transition :!class /Script/Engine.MaterialInstanceDynamic))
      (:Finished
        (if (not true)
          (Rendering|Material|SetMaterial 0 "/Game/Materials/M_Character.M_Character")))))
  (:Released
    (Variables|Default|SetisInvisible false)
    (Timeline|Opacity%20Change Reverse)))

(event Input|MouseEvents|RightMouseButton
  ;[1 1 1] Invisbility Logic
  (:Pressed
    (Variables|Default|SetisInvisible true)
    (Rendering|Material|SetMaterial 0 (Variables|Default|GettranslucentMaterial))
    (EventDispatchers|BindEventtoTriedInvisibility (delegate Custom|Tried%20Invisibility%20Event))
    (Default|CallTriedInvisibility)
    (bind _transition (Timeline|Opacity%20Change Play)
      (:Update
        (Rendering|Material|SetScalarParameterValue (Variables|Default|GettranslucentMaterial) "Opacity" _transition :!class /Script/Engine.MaterialInstanceDynamic))
      (:Finished
        (if (not true)
          (Rendering|Material|SetMaterial 0 "/Game/Materials/M_Character.M_Character")))))
  (:Released
    (Variables|Default|SetisInvisible false)
    (Timeline|Opacity%20Change Reverse)))

(fn ConstructionScript
  (bind _mesh (Variables|Character|GetMesh))
  (bind _returnvalue (Rendering|Material|CreateDynamicMaterialInstance 0 "/Game/Materials/M_Character_Trans.M_Character_Trans" :!class /Script/Engine.PrimitiveComponent))
  (Variables|Default|SettranslucentMaterial _returnvalue)
  (Rendering|Material|SetMaterial 0 "/Game/Materials/M_Character.M_Character")
  ;[1 1 1] Set up hand collsion
  (Class|SceneComponent|Attachto (Variables|Default|GetHandCollision_L) _mesh "hand_l" "SnapToTarget" true)
  (Class|SceneComponent|Attachto (Variables|Default|GetHandCollision_R) _mesh "hand_r" "SnapToTarget" true))

(fn SetIsPossessing
  (params (isPossessing :type Boolean))
  (Variables|Default|SetisPossessing isPossessing))

(fn EnableCharacter
  (params (Enable :type Boolean))
  (if Enable
    (Rendering|SetActorHiddenInGame false)
    (Collision|SetCollisionEnabled "QueryAndPhysics")
    (else
      (Rendering|SetActorHiddenInGame true)
      (Collision|SetCollisionEnabled "NoCollision"))))