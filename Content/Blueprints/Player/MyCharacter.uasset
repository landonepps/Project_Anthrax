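; Player character that can slash, turn invisible and possess objects, and creates the HUD on BeginPlay.
; Invisibility swaps to a dynamic translucent material faded by a timeline; slashing cancels and blocks it.
; Each tick highlights the PossessCapsule overlap nearest a fixed screen point as the Possess target, and interpolates the camera boom toward CameraTransform.
; Tick also polls health; while dead, it reapplies ragdoll and replays the death sound every frame.
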(event OnComponentEndOverlap(PossessCapsule)
  (params (OtherActor :type Actor%20Object%20Reference) (OtherComp :type Primitive%20Component%20Object%20Reference) (OtherBodyIndex :type Integer))
  ;[1 1 1] Disable Highlight on Objects
  (bind _aspossessable_object_p (Utilities|Casting|CastToPossessableObject_P OtherActor))
  (Default|SetHighlightActive _aspossessable_object_p false))

(event Custom|invisibilityChanged
  ;[1 1 1] Invisibility Logic
  (if (Variables|Default|GetisInvisible)
    (Rendering|Material|SetMaterial 0 (Variables|Default|GettranslucentMaterial))
    (EventDispatchers|BindEventtoTriedInvisibility (delegate Custom|Tried%20Invisibility%20Event))
    (Default|CallTriedInvisibility)
    (bind _transition (Timeline|Opacity%20Change Play)
      (:Update
        (Rendering|Material|SetScalarParameterValue (Variables|Default|GettranslucentMaterial) "Opacity" _transition :!class /Script/Engine.MaterialInstanceDynamic))
      (:Finished
        (if (not (Variables|Default|GetisInvisible))
          (Rendering|Material|SetMaterial 0 "/Game/Materials/M_Character.M_Character"))))
    (else
      (Timeline|Opacity%20Change Reverse))))

(event Custom|CheckPossession
  ;[1 1 1] Possession Logic With Highlight
  (bind (_outactors _returnvalue) (Class|KismetSystemLibrary|ComponentOverlapActorsNEW (Variables|Default|GetPossessCapsule) (Transformation|GetWorldTransform) (Utilities|Array|MakeArray "ObjectTypeQuery1") "/Game/Blueprints/PossessableObjects/PossessableObject_P.PossessableObject_P_C"))
  (Variables|Default|SetpossessableObjectDistFromScreenCenter 1000000)
  (for _array_element _outactors
    ;;[1 1 1] Loop over all Possessable Objects colliding with PossessCapsule and determine center-most object
    (bind _aspossessable_object_p (Utilities|Casting|CastToPossessableObject_P _array_element))
    (Default|SetHighlightActive _aspossessable_object_p false)
    (if (< (Math|Vector2D|Vector2DLength (- (.ScreenLocation (Class|PlayerController|ProjectWorldLocationtoScreen (Game|GetPlayerController 0) (Transformation|GetActorLocation _array_element))) "(X=700.000000,Y=700.000000)")) (Math|Conversions|ToFloat(Integer) (Variables|Default|GetpossessableObjectDistFromScreenCenter)))
      (Variables|Default|SetpossessableObjectDistFromScreenCenter (Math|Float|Floor (Math|Vector2D|Vector2DLength (- (.ScreenLocation (Class|PlayerController|ProjectWorldLocationtoScreen (Game|GetPlayerController 0) (Transformation|GetActorLocation _array_element))) "(X=700.000000,Y=700.000000)"))))
      (Variables|Default|SetSelected%20Possession%20Object _array_element)))
  (if _returnvalue
    (bind _aspossessable_object_p_2 (Utilities|Casting|CastToPossessableObject_P (Variables|Default|GetSelected%20Possession%20Object)))
    (Default|SetHighlightActive _aspossessable_object_p_2 true)))

(event Custom|Tried%20Invisibility%20Event
  ;[1 1 1] Invisibility Logic
)

(event Custom|set%20camera
  (params (transform :type Transform))
  (bind (_location _rotation) (Math|Transform|BreakTransform transform))
  (Transformation|SetWorldLocationAndRotation _location _rotation false))

(event Custom|Tried%20Possession%20Event
  ;[1 1 1] Possess selected object
)

(event Custom|Transition%20Camera
  (params (tranform :type Transform))
  (bind _cameraboom (Variables|Default|GetCameraBoom))
  ;[1 1 1] Transition Camera smoothly when possessing
  (Transformation|SetWorldLocation _cameraboom (Math|Interpolation|VInterpTo (Transformation|GetWorldLocation _cameraboom) (.Location (Math|Transform|BreakTransform tranform)) (Utilities|Time|GetWorldDeltaSeconds) (Variables|Default|GetcameraTransitionSpeed)) false))

(event EventTick
  (params (DeltaSeconds :type Float%20%28single-precision%29))
  ;[1 1 1] Event Tick
  (CallFunction|CheckPossession)
  (CallFunction|TransitionCamera (Transformation|GetWorldTransform (Variables|Default|Getcamera%20transform)))
  (CallFunction|CheckHealth)
  (CallFunction|CheckDead))

(event EventBeginPlay
  ;[1 1 1] Startup logic
  ;[1 1 1] HUD
  (bind _returnvalue (UserInterface|CreateWidget "/Game/UserInterface/BasicHUD.BasicHUD_C"))
  (UserInterface|Viewport|AddtoViewport _returnvalue)
  (if (not (Math|Vector|NotEqual(Vector) (Transformation|GetWorldLocation (Variables|Default|Getcamera%20transform)) "0, 0, 0" 0.0001))
    (Development|PrintString 0 (Utilities|String|Append (Utilities|String|Append (Utilities|String|MakeLiteralString "ERROR: ") (Utilities|GetDisplayName self)) "has no CameraDefaultPos"))))

(event Input|ActionEvents|InputActionPossess
  ;[1 1 1] Possess selected object
  (:Pressed
    (if (< (Variables|Default|GetpossessableObjectDistFromScreenCenter) 1000000)
      (Class|PossessableI|EnterPossession(Message) (Variables|Default|GetSelected%20Possession%20Object) (Game|Player|GetPlayerPawn 0))
      (EventDispatchers|BindEventtoTriedPossession (delegate Custom|Tried%20Possession%20Event))
      (Default|CallTriedPossession))))

(event Input|ActionEvents|InputActionGoInvisible
  ;[1 1 1] Invisibility Logic
  (:Pressed
    (if (not (Variables|Default|GetisSlashing))
      (Variables|Default|SetisInvisible true)
      (Rendering|Material|SetMaterial 0 (Variables|Default|GettranslucentMaterial))
      (EventDispatchers|BindEventtoTriedInvisibility (delegate Custom|Tried%20Invisibility%20Event))
      (Default|CallTriedInvisibility)
      (bind _transition (Timeline|Opacity%20Change Play)
        (:Update
          (Rendering|Material|SetScalarParameterValue (Variables|Default|GettranslucentMaterial) "Opacity" _transition :!class /Script/Engine.MaterialInstanceDynamic))
        (:Finished
          (if (not (Variables|Default|GetisInvisible))
            (Rendering|Material|SetMaterial 0 "/Game/Materials/M_Character.M_Character"))))))
  (:Released
    (Variables|Default|SetisInvisible false)
    (Timeline|Opacity%20Change Reverse)))

(event Input|GamepadEvents|GamepadRightTrigger
  ;[1 1 1] Slashing attack
  (:Pressed
    (Variables|Default|SetisSlashing true)
    ;[1 1 1] Invisibility Logic
    (Variables|Default|SetisInvisible false)
    (bind _transition (Timeline|Opacity%20Change Reverse)
      (:Update
        (Rendering|Material|SetScalarParameterValue (Variables|Default|GettranslucentMaterial) "Opacity" _transition :!class /Script/Engine.MaterialInstanceDynamic))
      (:Finished
        (if (not (Variables|Default|GetisInvisible))
          (Rendering|Material|SetMaterial 0 "/Game/Materials/M_Character.M_Character")))))
  (:Released
    (Variables|Default|SetisSlashing false)))

(event Input|MouseEvents|LeftMouseButton
  ;[1 1 1] Slashing attack
  (:Pressed
    (Variables|Default|SetisSlashing true)
    ;[1 1 1] Invisibility Logic
    (Variables|Default|SetisInvisible false)
    (bind _transition (Timeline|Opacity%20Change Reverse)
      (:Update
        (Rendering|Material|SetScalarParameterValue (Variables|Default|GettranslucentMaterial) "Opacity" _transition :!class /Script/Engine.MaterialInstanceDynamic))
      (:Finished
        (if (not (Variables|Default|GetisInvisible))
          (Rendering|Material|SetMaterial 0 "/Game/Materials/M_Character.M_Character")))))
  (:Released
    (Variables|Default|SetisSlashing false)))

(fn ConstructionScript
  (bind _returnvalue (Rendering|Material|CreateDynamicMaterialInstance 0 "/Game/Materials/M_Character_Trans.M_Character_Trans" :!class /Script/Engine.PrimitiveComponent))
  (Variables|Default|SettranslucentMaterial _returnvalue)
  (Rendering|Material|SetMaterial 0 "/Game/Materials/M_Character.M_Character"))

(fn SetIsPossessing
  (params (isPossessing :type Boolean))
  (Variables|Default|SetisPossessing isPossessing))

(fn EnableCharacter
  (params (Enable :type Boolean))
  (if Enable
    (Rendering|SetActorHiddenInGame false)
    (Collision|SetCollisionEnabled "QueryAndPhysics")
    (else
      (Rendering|SetActorHiddenInGame true)
      (Collision|SetCollisionEnabled "NoCollision"))))

(fn CheckDead
  (bind _mesh (Variables|Character|GetMesh))
  (if (Variables|Default|Getdead)
    (Class|GameplayStatics|PlaySoundAttached "/Game/Audio/DamageAudio/male_death1.male_death1" _mesh)
    (Physics|SetSimulatePhysics _mesh true)
    (Collision|SetCollisionEnabled (Variables|Default|GetCapsuleComponent) "NoCollision")))

(fn CheckHealth
  (if (<= (Variables|Default|Gethealth) 0.0)
    (Variables|Default|Setdead true)))

(fn GetHealth
  ;[1 1 1] Returns Health
  (return (Variables|Default|Gethealth)))

(fn TakeDamage
  (params (attackDamage :type Float%20%28single-precision%29))
  (Variables|Default|SetHealth (- (Variables|Default|GetHealth) attackDamage))
  (Class|GameplayStatics|PlaySoundAttached "/Game/Audio/DamageAudio/low_grunt1.low_grunt1" (Variables|Character|GetMesh))
  (return true))